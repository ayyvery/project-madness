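; BP_SpellIce_Child is an ice spear spell actor, derived from a parent Blueprint, that damages whatever it overlaps.
; On overlap it spawns a flash emitter and explosion sound at its Collision component, applies fixed damage to the other actor and destroys itself.
; A BeginPlay delay destroys it after four seconds, though the graph comment says five.
; Its construction script only calls the parent's.
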(event `self.ReceiveBeginPlay`
  ;[1 1 1] destroy after 5 seconds
  (`KismetSystemLibrary.Delay` 4.0)
  (`self.K2_DestroyActor`))

(event `self.ReceiveActorBeginOverlap`
  (params (OtherActor :type "Actor Object Reference"))
  (bind _location (.location (`SceneComponent.K2_GetComponentToWorld` (`self.Collision`))))
  ;[1 1 1] explosion after overlaping and destroying
  (`GameplayStatics.SpawnEmitterAtLocation` "/Game/NewFolder/AdvancedMagicFX13/Particles/P_ky_flash2.P_ky_flash2" _location (.rotation (`SceneComponent.K2_GetComponentToWorld` (`self.Collision`))) (.scale (`SceneComponent.K2_GetComponentToWorld` (`self.Collision`))))
  (`GameplayStatics.PlaySoundAtLocation` "/Game/ProjectMadness/StarterContent/Audio/Explosion01.Explosion01" _location (struct) 1.0 1.0 0.0 null null null)
  (`GameplayStatics.ApplyDamage` OtherActor 100.0 null null "/Script/Engine.DamageType")
  (`self.K2_DestroyActor`))

(fn `UserConstructionScript`
  (`parent.UserConstructionScript`))