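; Energy burst spell actor, a child Blueprint that reacts when it overlaps another actor.
; Every overlap spawns a thunder hit emitter and explosion sound at the Fireball component's location.
; If the other actor is a DefaultEnemy within FireDistance, it gets a single movement input pointing away from the fireball, then the spell destroys itself.
; Other overlaps leave the spell alive, and construction only calls the parent script.
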(event `self.ReceiveActorBeginOverlap`
  (params (OtherActor :type "Actor Object Reference"))
  (bind _location (.location (`SceneComponent.K2_GetComponentToWorld` (`self.Fireball`))))
  (`GameplayStatics.SpawnEmitterAtLocation` "/Game/NewFolder/AdvancedMagicFX12/particles/P_ky_hit_thunder.P_ky_hit_thunder" _location (.rotation (`SceneComponent.K2_GetComponentToWorld` (`self.Fireball`))))
  (`GameplayStatics.PlaySoundAtLocation` "/Game/ProjectMadness/StarterContent/Audio/Explosion01.Explosion01" _location (struct) 1.0 1.0 0.0 null null null)
  (bind _asdefault_enemy (cast `/Game/ProjectMadness/Enemies/Default/DefaultEnemy` OtherActor))
  (bind _returnvalue (`self.K2_GetActorLocation` _asdefault_enemy))
  (if (< (`KismetMathLibrary.Vector_Distance` _location _returnvalue) (`self.FireDistance`))
    (`Pawn.AddMovementInput` _asdefault_enemy (`KismetMathLibrary.GetForwardVector` (`KismetMathLibrary.FindLookAtRotation` _location _returnvalue)) 1.0 false)
    (`self.K2_DestroyActor`)))

(fn `UserConstructionScript`
  (`parent.UserConstructionScript`))