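; BP_BurstSplash is an Energy Burst spell actor that pushes on hit through forced movement input, then destroys itself.
; When its Sphere component hits, it compares a distance against FireDistance and applies scaled input to the hit actor's Instigator.
; Both the distance check and look-at direction use the splash's own location at each end, so the distance is zero and the direction ignores the hit actor.
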(event `self.Sphere.OnComponentHit`
  (params (HitComponent :type "PrimitiveComponent Object Reference") (OtherActor :type "Actor Object Reference") (OtherComp :type "PrimitiveComponent Object Reference") (NormalImpulse :type "Vector Structure") (Hit :type "HitResult Structure (by ref)"))
  (bind _returnvalue (`self.K2_GetActorLocation`))
  (bind _location (`self.Location`))
  (set `self.Location` (`self.K2_GetActorLocation`))
  (if (< (`KismetMathLibrary.Vector_Distance` _location _returnvalue) (`self.FireDistance`))
    (`Pawn.AddMovementInput` (`Actor.Instigator` OtherActor) (`KismetMathLibrary.GetForwardVector` (`KismetMathLibrary.FindLookAtRotation` _location _returnvalue)) 10.0 true)
    (`self.K2_DestroyActor`)))

(fn `UserConstructionScript`)