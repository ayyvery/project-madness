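; BP_Platform is an arena platform that rises from world Z zero to its placed height when the game starts.
; BeginPlay stores the Platform component's world Z in Hight, then snaps it to zero while keeping X and Y.
; Tick eases Z back toward Hight every frame with FInterpTo at InterpSpeed, moving with sweep on.
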(event `self.ReceiveBeginPlay`
  (bind _platform (`self.platform`))
  ;[1 1 1] when game starts put all platforms to 0 in z
  (set `self.hight` (.z (`SceneComponent.K2_GetComponentLocation` _platform)))
  (`SceneComponent.K2_SetWorldLocation` _platform (`KismetMathLibrary.MakeVector` (.x (`SceneComponent.K2_GetComponentLocation` _platform)) (.y (`SceneComponent.K2_GetComponentLocation` _platform))) false false))

(event `self.ReceiveTick`
  (params (DeltaSeconds :type "Float (single-precision)"))
  (bind _platform (`self.platform`))
  ;[1 1 1] lifting platforms
  (`SceneComponent.K2_SetWorldLocation` _platform (`KismetMathLibrary.MakeVector` (.x (`SceneComponent.K2_GetComponentLocation` _platform)) (.y (`SceneComponent.K2_GetComponentLocation` _platform)) (`KismetMathLibrary.FInterpTo` (.z (`SceneComponent.K2_GetComponentLocation` _platform)) (`self.hight`) (`GameplayStatics.GetWorldDeltaSeconds`) (`self.InterpSpeed`))) true false))

(fn `UserConstructionScript`)