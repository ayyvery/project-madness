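; BP_Camicadse is a kamikaze sphere enemy that chases the player and blows itself up at close range.
; Pawn sensing locks onto the first ThirdPersonCharacter seen and turns the eye's dynamic material red.
; Tick moves it toward the target with smoothed rotation, and within range triggers a one-time sound, delay and BP_Explosion spawn.
; Lethal damage explodes it immediately and heals the target by an HP award.
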(event `Explode`
  (bind _returnvalue (`SceneComponent.K2_GetComponentLocation` (`self.CapsuleComponent`)))
  ;[1 1 1] Expload
  (`GameplayStatics.PlaySoundAtLocation` "/Game/ProjectMadness/Enemies/sphere/PreExplosion.PreExplosion" _returnvalue (struct) 1.0 1.0 0.0 null null null)
  (`KismetSystemLibrary.Delay` 2.0)
  (`|SpawnActorFromClass` "/Game/ProjectMadness/Enemies/sphere/BP_Explosion.BP_Explosion_C" (`KismetMathLibrary.MakeTransform` _returnvalue) "Undefined" "OverrideRootScale" null null)
  (`self.K2_DestroyActor`))

(event `self.ReceiveBeginPlay`
  (bind _eye (`self.eye`))
  ;[1 1 1] ApplyMaterialInstance
  (bind _returnvalue (`PrimitiveComponent.CreateDynamicMaterialInstance` _eye 0 "/Game/ProjectMadness/Enemies/star/base/Light.Light" "None"))
  (set `self.MaterialInstance` _returnvalue)
  (`PrimitiveComponent.SetMaterial` _eye 1 null))

(event `self.ReceiveTick`
  (params (DeltaSeconds :type "Float (single-precision)"))
  ;[1 1 1] MovingAndExpload
  (bind _target (`self.Target`)
    (:`then`
      (if (> (`self.GetDistanceTo` _target) (`self.ExploadDistance`))
        _
        (elif (not (`self.once`))
          (`self.Explode`)
          (set `self.once` true)))
      (bind _returnvalue (`KismetMathLibrary.FindLookAtRotation` (`self.K2_GetActorLocation`) (+ (`self.K2_GetActorLocation` _target) (0.0 0.0 50.0))))
      (`self.AddMovementInput` (`KismetMathLibrary.GetForwardVector` _returnvalue))
      (bind (_returnvalue_roll _returnvalue_pitch _returnvalue_yaw) (`KismetMathLibrary.BreakRotator` (`KismetMathLibrary.RLerp` (`self.K2_GetActorRotation`) _returnvalue 0.1 true)))
      (`self.K2_SetActorRotation` (`KismetMathLibrary.MakeRotator` _returnvalue_roll _returnvalue_pitch _returnvalue_yaw)))
    (:`else`)))

(event `self.PawnSensing.OnSeePawn`
  (params (Pawn :type "Pawn Object Reference"))
  ;[1 1 1] MovingAndExpload
  ;;[1 1 1] OnSeePawn
  (`self.Target`
    (:`then`)
    (:`else`
      (bind _asthird_person_character (cast `/Game/ProjectMadness/ThirdPersonBP/Blueprints/ThirdPersonCharacter` Pawn))
      (set `self.Target` _asthird_person_character)
      (`self.BattleMod_On`))))

(event `self.ReceiveAnyDamage`
  (params (Damage :type "Float (single-precision)") (DamageType :type "DamageType Object Reference") (InstigatedBy :type "Controller Object Reference") (DamageCauser :type "Actor Object Reference"))
  (bind _returnvalue (- (`self.HP`) Damage))
  ;[1 1 1] Death
  (if (> _returnvalue 0.0)
    (set `self.HP` _returnvalue)
    (else
      (`|SpawnActorFromClass` "/Game/ProjectMadness/Enemies/sphere/BP_Explosion.BP_Explosion_C" (`KismetMathLibrary.MakeTransform` (`SceneComponent.K2_GetComponentLocation` (`self.CapsuleComponent`))) "Undefined" "OverrideRootScale" null null)
      (`self.K2_DestroyActor`)
      (`/Game/ProjectMadness/ThirdPersonBP/Blueprints/ThirdPersonCharacter.Heal` (`self.Target`) (`self.HP_Award`)))))

(fn `BattleMod_Off`
  (`KismetSystemLibrary.PrintString` "Battle mod off" true true (struct :`G` 0.244543 :`B` 1.0 :`A` 1.0))
  (`MaterialInstanceDynamic.SetVectorParameterValue` (`self.MaterialInstance`) "Color" (struct :`B` 1.0 :`A` 1.0))
  (set `self.BattleMod` false))

(fn `BattleMod_On`
  (`KismetSystemLibrary.PrintString` "Battle mod on" true true (struct :`R` 1.0 :`B` 0.027538 :`A` 1.0))
  (`MaterialInstanceDynamic.SetVectorParameterValue` (`self.MaterialInstance`) "Color" (struct :`R` 1.0 :`A` 1.0))
  (set `self.BattleMod` true))

(fn `UserConstructionScript`)