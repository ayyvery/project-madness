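; BP_StarManecen is a star enemy with a spinning body, a glowing eye and four laser emitters.
; BeginPlay creates the eye's dynamic material; Tick rotates the body and alternates its "Param" scalar each frame, as the trailing Delay gates nothing.
; BattlemodOn and BattlemodOff turn the eye red or blue with debug prints.
; Fire spawns a Laser at each of four arrow components; no calls to these functions appear here.
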(event `self.ReceiveBeginPlay`
  (bind _star_eye (`self.star eye`))
  ;[1 1 1] BeginPlay
  (bind _returnvalue (`PrimitiveComponent.CreateDynamicMaterialInstance` _star_eye 0 "/Game/ProjectMadness/Enemies/star/base/Light.Light" "None"))
  (bind _output_get (set `self.MaterialInstance` _returnvalue))
  (`PrimitiveComponent.SetMaterial` _star_eye 1 _output_get))

(event `self.ReceiveTick`
  (params (DeltaSeconds :type "Float (single-precision)"))
  ;[1 1 1] EyePulse
  (`SceneComponent.K2_AddLocalRotation` (`self.body`) (struct :`Pitch` 0.2) false false)
  (if (`self.Color`)
    (`MaterialInstanceDynamic.SetScalarParameterValue` (`self.MaterialInstance`) "Param" 20.0)
    (else
      (`MaterialInstanceDynamic.SetScalarParameterValue` (`self.MaterialInstance`) "Param" 30.0)))
  (set `self.Color` (not (`self.Color`)))
  (`KismetSystemLibrary.Delay` 1.0))

(fn `battlemod_off`
  (`KismetSystemLibrary.PrintString` "Battle mod off" true true (struct :`G` 0.244543 :`B` 1.0 :`A` 1.0))
  (`MaterialInstanceDynamic.SetVectorParameterValue` (`self.MaterialInstance`) "Color" (struct :`B` 1.0 :`A` 1.0)))

(fn `battlemod_on`
  (`KismetSystemLibrary.PrintString` "Battle mod on" true true (struct :`R` 1.0 :`B` 0.027538 :`A` 1.0))
  (`MaterialInstanceDynamic.SetVectorParameterValue` (`self.MaterialInstance`) "Color" (struct :`R` 1.0 :`A` 1.0)))

(fn `fire`
  (`|SpawnActorFromClass` "/Game/ProjectMadness/Enemies/star/laser/laser.laser_C" (`SceneComponent.K2_GetComponentToWorld` (`self.Arrow1`)) "AlwaysSpawn" "OverrideRootScale" null null)
  (`|SpawnActorFromClass` "/Game/ProjectMadness/Enemies/star/laser/laser.laser_C" (`SceneComponent.K2_GetComponentToWorld` (`self.Arrow2`)) "AlwaysSpawn" "OverrideRootScale" null null)
  (`|SpawnActorFromClass` "/Game/ProjectMadness/Enemies/star/laser/laser.laser_C" (`SceneComponent.K2_GetComponentToWorld` (`self.Arrow3`)) "AlwaysSpawn" "OverrideRootScale" null null)
  (`|SpawnActorFromClass` "/Game/ProjectMadness/Enemies/star/laser/laser.laser_C" (`SceneComponent.K2_GetComponentToWorld` (`self.Arrow4`)) "AlwaysSpawn" "OverrideRootScale" null null))

(fn `UserConstructionScript`)