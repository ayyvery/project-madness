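; Star enemy that turns to face the player and teleports at random within a fixed volume.
; A self-recalling delay loop smoothly rotates the body toward the player, while a timer repeats teleports with flash effects when allowed.
; Damage switches on battle mode, turning the eye's dynamic material red, and reduces HP until the actor is destroyed.
; A four-arrow laser volley is defined but its only call is disconnected.
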(event `self.ReceiveBeginPlay`
  (bind _star_eye (`self.star eye`))
  ;[1 1 1] BeginPlay
  (bind _asthird_person_character (cast `/Game/ProjectMadness/ThirdPersonBP/Blueprints/ThirdPersonCharacter` (`GameplayStatics.GetPlayerCharacter` 0)))
  (set `self.As Third Person Character` _asthird_person_character)
  (`self.teleport`)
  (bind _returnvalue (`PrimitiveComponent.CreateDynamicMaterialInstance` _star_eye 0 "/Game/ProjectMadness/Enemies/star/base/Light.Light" "None"))
  (bind _output_get (set `self.NewVar_3` _returnvalue))
  (`PrimitiveComponent.SetMaterial` _star_eye 1 _output_get)
  (`self.facetoplayer`))

(event `self.ReceiveTick`
  (params (DeltaSeconds :type "Float (single-precision)"))
  ;[1 1 1] FceToPlayer
)

(event `self.ReceiveAnyDamage`
  (params (Damage :type "Float (single-precision)") (DamageType :type "DamageType Object Reference") (InstigatedBy :type "Controller Object Reference") (DamageCauser :type "Actor Object Reference"))
  ;[1 1 1] Death
  (`self.battlemod_on`)
  (if true
    (if (<= (- (`self.HP`) Damage) 0.0)
      (`self.K2_DestroyActor`)
      (else
        (set `self.HP` (- (`self.HP`) Damage))))))

(event `facetoplayer`
  (bind _body (`self.body`))
  ;[1 1 1] Face to player
  (`SceneComponent.K2_SetWorldRotation` (`self.body`) (`KismetMathLibrary.RInterpTo` (`SceneComponent.K2_GetComponentRotation` _body) (`KismetMathLibrary.MakeRotator` (.roll (`KismetMathLibrary.FindLookAtRotation` (`SceneComponent.K2_GetComponentLocation` _body) (+ (`self.K2_GetActorLocation` (`self.As Third Person Character`)) (0.0 0.0 50.0)))) (+ (.pitch (`KismetMathLibrary.FindLookAtRotation` (`SceneComponent.K2_GetComponentLocation` _body) (+ (`self.K2_GetActorLocation` (`self.As Third Person Character`)) (0.0 0.0 50.0)))) 0.0) (+ (.yaw (`KismetMathLibrary.FindLookAtRotation` (`SceneComponent.K2_GetComponentLocation` _body) (+ (`self.K2_GetActorLocation` (`self.As Third Person Character`)) (0.0 0.0 50.0)))) 90.0)) (`GameplayStatics.GetWorldDeltaSeconds`) 15.0) false false)
  (`KismetSystemLibrary.Delay` 0.001)
  (`self.facetoplayer`))

(event `teleport`
  (bind _returnvalue (`KismetMathLibrary.MakeVector` (`KismetMathLibrary.RandomFloatInRange` -3723.748779 3733.419434) (`KismetMathLibrary.RandomFloatInRange` -3740.938965 3677.426025) (`KismetMathLibrary.RandomFloatInRange` 616.955383 3060.625488)))
  ;[1 1 1] Teleport
  (if (`self.CanTeleport`)
    (`GameplayStatics.SpawnEmitterAtLocation` "/Game/NewFolder/AdvancedMagicFX13/Particles/P_ky_flash1.P_ky_flash1" (`SceneComponent.K2_GetComponentLocation` (`self.body`)))
    (`SceneComponent.K2_SetWorldLocation` (`self.body`) _returnvalue false true)
    (`GameplayStatics.SpawnEmitterAtLocation` "/Game/NewFolder/AdvancedMagicFX13/Particles/P_ky_flash1.P_ky_flash1" _returnvalue)
    (`KismetSystemLibrary.K2_SetTimerDelegate` (delegate `teleport`) (`self.TeleportCooldown`) true)))

(fn `battlemod_off`
  (`KismetSystemLibrary.PrintString` "Battle mod off" true true (struct :`G` 0.244543 :`B` 1.0 :`A` 1.0))
  (`MaterialInstanceDynamic.SetVectorParameterValue` (`self.NewVar_3`) "Color" (struct :`B` 1.0 :`A` 1.0))
  (set `self.Battle_mod` false))

(fn `battlemod_on`
  (`KismetSystemLibrary.PrintString` "Battle mod on" true true (struct :`R` 1.0 :`B` 0.027538 :`A` 1.0))
  (`MaterialInstanceDynamic.SetVectorParameterValue` (`self.NewVar_3`) "Color" (struct :`R` 1.0 :`A` 1.0))
  (set `self.Battle_mod` true))

(fn `fire`
  (`|SpawnActorFromClass` "/Game/ProjectMadness/Enemies/star/laser/laser.laser_C" (`SceneComponent.K2_GetComponentToWorld` (`self.Arrow1`)) "Undefined" "OverrideRootScale" null null)
  (`|SpawnActorFromClass` "/Game/ProjectMadness/Enemies/star/laser/laser.laser_C" (`SceneComponent.K2_GetComponentToWorld` (`self.Arrow2`)) "Undefined" "OverrideRootScale" null null)
  (`|SpawnActorFromClass` "/Game/ProjectMadness/Enemies/star/laser/laser.laser_C" (`SceneComponent.K2_GetComponentToWorld` (`self.Arrow3`)) "Undefined" "OverrideRootScale" null null)
  (`|SpawnActorFromClass` "/Game/ProjectMadness/Enemies/star/laser/laser.laser_C" (`SceneComponent.K2_GetComponentToWorld` (`self.Arrow4`)) "Undefined" "OverrideRootScale" null null))

(fn `UserConstructionScript`)