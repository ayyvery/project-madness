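; BP_cube is an enemy cube that spins one mesh part and spawns Laser actors from its Arrow component.
; Tick drives both the rotation and a frame-counted fire delay, so it keeps firing regardless of battle mode and at a rate tied to framerate.
; Each actor overlap toggles battle mode, recoloring a dynamic Light material red or blue with a debug print; switching on also fires immediately.
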(event `self.ReceiveBeginPlay`
  (bind _cubbe_roundcube_001 (`self.CUBBE_Roundcube_001`))
  ;[1 1 1] apply dyn mat
  (bind _returnvalue (`PrimitiveComponent.CreateDynamicMaterialInstance` _cubbe_roundcube_001 0 "/Game/ProjectMadness/Enemies/star/base/Light.Light" "None"))
  (bind _output_get (set `self.DynamicMaterial` _returnvalue))
  (`PrimitiveComponent.SetMaterial` _cubbe_roundcube_001 1 _output_get))

(event `self.ReceiveActorBeginOverlap`
  (params (OtherActor :type "Actor Object Reference"))
  ;[1 1 1] Change battle mod
  (if (`self.BattleMod`)
    (`self.BattleModOff`)
    (else
      (`self.BattleModOn`))))

(event `self.ReceiveTick`
  (params (DeltaSeconds :type "Float (single-precision)"))
  ;[1 1 1] rotate and fire
  (`SceneComponent.K2_AddLocalRotation` (`self.CUBBE_Roundcube_004`) (struct :`Yaw` 1.0) false false)
  (if (< (`self.FireDelay`) 20)
    (set `self.FireDelay` (+ (`self.FireDelay`) 1))
    (else
      (set `self.FireDelay` 0)
      (`self.fire`))))

(fn `BattleModOff`
  (`KismetSystemLibrary.PrintString` "Battle mod off" true true (struct :`G` 0.244543 :`B` 1.0 :`A` 1.0))
  (`MaterialInstanceDynamic.SetVectorParameterValue` (`self.DynamicMaterial`) "Color" (struct :`B` 1.0 :`A` 1.0))
  (set `self.BattleMod` false))

(fn `BattleModOn`
  (`KismetSystemLibrary.PrintString` "Battle mod on" true true (struct :`R` 1.0 :`B` 0.027538 :`A` 1.0))
  (`MaterialInstanceDynamic.SetVectorParameterValue` (`self.DynamicMaterial`) "Color" (struct :`R` 1.0 :`A` 1.0))
  (set `self.BattleMod` true)
  (`self.fire`))

(fn `Fire`
  (`|SpawnActorFromClass` "/Game/ProjectMadness/Enemies/star/laser/laser.laser_C" (`SceneComponent.K2_GetComponentToWorld` (`self.Arrow`)) "AlwaysSpawn" "OverrideRootScale" null null))

(fn `UserConstructionScript`)